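; Player tank Blueprint that routes input to movement, aiming and camera controls.
; On BeginPlay it hands the left and right tracks to TankMovement, and the turret and barrel to TankAiming.
; Drive and turn axes become movement intentions on TankMovement, and Fire calls TankAiming.
; Camera input yaws the Horizontal component and pitches the SpringArm separately, using relative rotations.
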(event EventBeginPlay
  ;[1 1 1] BeginPlay
  (Class|TankMovementComponent|Initialise (Variables|Default|GetTankMovement) (Variables|Default|GetTrack_Right) (Variables|Default|GetTrack_Left))
  (Class|TankAimingComponent|Initialise (Variables|Default|GetTankAiming) (Variables|Default|GetTurret) (Variables|Default|GetBarrel)))

(event Input|ActionEvents|InputActionFire
  (params (Key :type Key%20Structure :default "None"))
  ;[1 1 1] Input_Firing
  (:Pressed
    (Class|TankAimingComponent|Fire (Variables|Default|GetTankAiming))))

(event Input|AxisEvents|InputAxisHorizontal_Aim
  (params (AxisValue :type Float%20%28single-precision%29))
  ;[1 1 1] Input_Camera
  (Transformation|AddRelativeRotation (Variables|Default|GetHorizontal) (Math|Rotator|MakeRotator 0.0 0.0 AxisValue) false false))

(event Input|AxisEvents|InputAxisVertical_Aim
  (params (AxisValue :type Float%20%28single-precision%29))
  ;[1 1 1] Input_Camera
  (Transformation|AddRelativeRotation (Variables|Default|GetSpringArm) (Math|Rotator|MakeRotator 0.0 AxisValue 0.0) false false))

(event Input|AxisEvents|InputAxisTurnRight
  (params (AxisValue :type Float%20%28single-precision%29))
  ;[1 1 1] Input_Movement
  (Class|TankMovementComponent|MoveRightIntention (Variables|Default|GetTankMovement) AxisValue))

(event Input|AxisEvents|InputAxisTurnLeft
  (params (AxisValue :type Float%20%28single-precision%29))
  ;[1 1 1] Input_Movement
  (Class|TankMovementComponent|MoveRightIntention (Variables|Default|GetTankMovement) AxisValue))

(event Input|AxisEvents|InputAxisForward
  (params (AxisValue :type Float%20%28single-precision%29))
  ;[1 1 1] Input_Movement
  (Class|TankMovementComponent|MoveForwardIntention (Variables|Default|GetTankMovement) AxisValue))

(event Input|AxisEvents|InputAxisBackward
  (params (AxisValue :type Float%20%28single-precision%29))
  ;[1 1 1] Input_Movement
  (Class|TankMovementComponent|MoveForwardIntention (Variables|Default|GetTankMovement) AxisValue))

(fn ConstructionScript)